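; BP_GarageDoor is a one-shot hit trigger that clears a set of doors and labels, then reveals or repositions area signage.
; When its static mesh is hit, it destroys the referenced Text and Door actors.
; It then teleports the Basement, Electrical, Storage and Security text actors straight up by a fixed offset and destroys itself.
; All logic runs in that single hit event, with an empty construction script.
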(event `self.StaticMeshComponent.OnComponentHit`
  (params (HitComponent :type "PrimitiveComponent Object Reference") (OtherActor :type "Actor Object Reference") (OtherComp :type "PrimitiveComponent Object Reference") (NormalImpulse :type "Vector Structure") (Hit :type "HitResult Structure (by ref)"))
  (bind _basement_text (`self.Basement Text`))
  (bind _security_text (`self.Security Text`))
  (bind _electical_text (`self.Electical Text`))
  (bind _storage_text (`self.Storage Text`))
  (`self.K2_DestroyActor` (`self.Text_1`))
  (`self.K2_DestroyActor` (`self.Text_2`))
  (`self.K2_DestroyActor` (`self.Text_3`))
  (`self.K2_DestroyActor` (`self.Text_4`))
  (`self.K2_DestroyActor` (`self.Text_5`))
  (`self.K2_DestroyActor` (`self.Door_1`))
  (`self.K2_DestroyActor` (`self.Door_2`))
  (`self.K2_DestroyActor` (`self.Door_3`))
  (`self.K2_DestroyActor` (`self.Door_4`))
  (`self.K2_SetActorLocation` _basement_text (+ (`self.K2_GetActorLocation` _basement_text) (`KismetMathLibrary.MakeVector` 0.0 0.0 400.0)) false true)
  (`self.K2_SetActorLocation` _electical_text (+ (`self.K2_GetActorLocation` _electical_text) (`KismetMathLibrary.MakeVector` 0.0 0.0 400.0)) false true)
  (`self.K2_SetActorLocation` _storage_text (+ (`self.K2_GetActorLocation` _storage_text) (`KismetMathLibrary.MakeVector` 0.0 0.0 400.0)) false true)
  (`self.K2_SetActorLocation` _security_text (+ (`self.K2_GetActorLocation` _security_text) (`KismetMathLibrary.MakeVector` 0.0 0.0 400.0)) false true)
  (`self.K2_DestroyActor`))

(fn `UserConstructionScript`)