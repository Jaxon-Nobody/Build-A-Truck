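; Ceiling light actor that turns white and fades up from dark when its TargetActor begins an overlap.
; The construction script applies the configured intensity and colour to the point light.
; ActivateLightRamp stores the start and target intensity, and Tick blends between them over TimePeriod with a cubic ease-in.
; A near-zero period completes the ramp on the next tick.
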(event `self.Target Actor.OnActorBeginOverlap`
  (params (OverlappedActor :type "Actor Object Reference") (OtherActor :type "Actor Object Reference"))
  (`LightComponent.SetIntensity` (`self.PointLight`) 0.0)
  (`self.Activate Light Ramp` (`self.Target Intesity`) (`self.Time Period`))
  (`LightComponent.SetLightColor` (`self.PointLight`) (struct :`R` 1.0 :`G` 1.0 :`B` 1.0 :`A` 1.0) true))

(event `self.ReceiveTick`
  (params (DeltaSeconds :type "Float (single-precision)"))
  (bind _pointlight (`self.PointLight`))
  (if (`self.Changing`)
    (bind _output_get (set `self.Lerp Factor` (+ (`self.Lerp Factor`) (/ DeltaSeconds (`self.Time Period`)))))
    (if (>= _output_get 1.0)
      (`LightComponent.SetIntensity` _pointlight (`self.Target Intesity`))
      (set `self.Changing` false)
      (else
        (`LightComponent.SetIntensity` _pointlight (`KismetMathLibrary.Lerp` (`self.Start Intensity`) (`self.Target Intesity`) (`KismetMathLibrary.MultiplyMultiply_FloatFloat` (`self.Lerp Factor`) 3.0)))))))

(fn `Activate Light Ramp`
  (params (Intesity :type "Float (double-precision)") (`Time Period` :type "Float (double-precision)"))
  (set `self.Target Intesity` Intesity)
  (set `self.Time Period` `Time Period`)
  (set `self.Start Intensity` (`LightComponentBase.Intensity` (`self.PointLight`)))
  (set `self.Changing` true)
  (if (< (`self.Time Period`) 0.0001)
    (set `self.Lerp Factor` 1.0)
    (else
      (set `self.Lerp Factor` 0.0))))

(fn `UserConstructionScript`
  (bind _pointlight (`self.PointLight`))
  (`LightComponent.SetIntensity` _pointlight (`self.Intensity`))
  (`LightComponent.SetLightColor` _pointlight (`self.Colour`) true))