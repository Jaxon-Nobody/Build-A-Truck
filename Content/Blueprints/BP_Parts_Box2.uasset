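; BP_Parts_Box2 is a one-shot hit trigger that clears a part and a set of second-floor actors from the level.
; Any hit on its Cube component teleports the referenced Cross actor a short distance along negative world X, without sweeping.
; It then destroys the referenced Part, each individually referenced SecondFloor actor and finally itself, with no check on what caused the hit.
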(event `self.Cube.OnComponentHit`
  (params (HitComponent :type "PrimitiveComponent Object Reference") (OtherActor :type "Actor Object Reference") (OtherComp :type "PrimitiveComponent Object Reference") (NormalImpulse :type "Vector Structure") (Hit :type "HitResult Structure (by ref)"))
  (bind _cross (`self.Cross`))
  (`self.K2_SetActorLocation` _cross (+ (`self.K2_GetActorLocation` _cross) (`KismetMathLibrary.MakeVector` -13.0)) false true)
  (`self.K2_DestroyActor` (`self.Part`))
  (`self.K2_DestroyActor` (`self.Second Floor`))
  (`self.K2_DestroyActor` (`self.Second Floor_0`))
  (`self.K2_DestroyActor` (`self.Second Floor_1`))
  (`self.K2_DestroyActor` (`self.Second Floor_3`))
  (`self.K2_DestroyActor` (`self.Second Floor_4`))
  (`self.K2_DestroyActor` (`self.Second Floor_5`))
  (`self.K2_DestroyActor` (`self.Second Floor_6`))
  (`self.K2_DestroyActor` (`self.Second Floor_7`))
  (`self.K2_DestroyActor` (`self.Second Floor_8`))
  (`self.K2_DestroyActor` (`self.Second Floor_9`))
  (`self.K2_DestroyActor` (`self.Second Floor_10`))
  (`self.K2_DestroyActor` (`self.Second Floor_11`))
  (`self.K2_DestroyActor` (`self.Second Floor_12`))
  (`self.K2_DestroyActor` (`self.Second Floor_13`))
  (`self.K2_DestroyActor` (`self.Second Floor_14`))
  (`self.K2_DestroyActor` (`self.Second Floor_2`))
  (`self.K2_DestroyActor`))

(fn `UserConstructionScript`)