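; BP_Button2 is an overlap-triggered button that visually switches itself and three linked target actors on and off.
; When its Box is entered or exited, the Cube swaps to the on or off material.
; The same material then spreads to each target actor's first primitive component in sequence, with short delays creating a staggered chain effect.
; There is no filter on the overlapping actor, and only materials change.
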(event `self.Box.OnComponentBeginOverlap`
  (params (OverlappedComponent :type "PrimitiveComponent Object Reference") (OtherActor :type "Actor Object Reference") (OtherComp :type "PrimitiveComponent Object Reference") (OtherBodyIndex :type Integer) (bFromSweep :type Boolean) (SweepResult :type "HitResult Structure (by ref)"))
  (`PrimitiveComponent.SetMaterial` (`self.Cube`) 0 "/Game/Materials/M_ButtonOn.M_ButtonOn")
  (`KismetSystemLibrary.Delay` 0.2)
  (`PrimitiveComponent.SetMaterial` (`self.GetComponentByClass` (`self.Target Actor1`) "/Script/Engine.PrimitiveComponent") 0 "/Game/Materials/M_ButtonOn.M_ButtonOn")
  (`KismetSystemLibrary.Delay` 0.2)
  (`PrimitiveComponent.SetMaterial` (`self.GetComponentByClass` (`self.Target Actor2`) "/Script/Engine.PrimitiveComponent") 0 "/Game/Materials/M_ButtonOn.M_ButtonOn")
  (`KismetSystemLibrary.Delay` 0.2)
  (`PrimitiveComponent.SetMaterial` (`self.GetComponentByClass` (`self.Target Actor3`) "/Script/Engine.PrimitiveComponent") 0 "/Game/Materials/M_ButtonOn.M_ButtonOn"))

(event `self.Box.OnComponentEndOverlap`
  (params (OverlappedComponent :type "PrimitiveComponent Object Reference") (OtherActor :type "Actor Object Reference") (OtherComp :type "PrimitiveComponent Object Reference") (OtherBodyIndex :type Integer))
  (`PrimitiveComponent.SetMaterial` (`self.Cube`) 0 "/Game/Materials/M_ButtonOff.M_ButtonOff")
  (`KismetSystemLibrary.Delay` 0.2)
  (`PrimitiveComponent.SetMaterial` (`self.GetComponentByClass` (`self.Target Actor1`) "/Script/Engine.PrimitiveComponent") 0 "/Game/Materials/M_ButtonOff.M_ButtonOff")
  (`KismetSystemLibrary.Delay` 0.2)
  (`PrimitiveComponent.SetMaterial` (`self.GetComponentByClass` (`self.Target Actor2`) "/Script/Engine.PrimitiveComponent") 0 "/Game/Materials/M_ButtonOff.M_ButtonOff")
  (`KismetSystemLibrary.Delay` 0.2)
  (`PrimitiveComponent.SetMaterial` (`self.GetComponentByClass` (`self.Target Actor3`) "/Script/Engine.PrimitiveComponent") 0 "/Game/Materials/M_ButtonOff.M_ButtonOff"))

(fn `UserConstructionScript`)