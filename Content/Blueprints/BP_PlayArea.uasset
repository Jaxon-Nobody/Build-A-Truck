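; BP_PlayArea is a boundary volume that returns actors leaving it to a spawn point.
; When an actor ends overlap with the collision component, it teleports to an offset from the Spawn actor's location.
; If the relocated actor is then beyond a set distance from the Platform, the Platform also teleports back to its StartPosition actor.
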(event `self.CollisionComponent.OnComponentEndOverlap`
  (params (OverlappedComponent :type "PrimitiveComponent Object Reference") (OtherActor :type "Actor Object Reference") (OtherComp :type "PrimitiveComponent Object Reference") (OtherBodyIndex :type Integer))
  (bind _output_get (set `self.Character` OtherActor))
  (`self.K2_SetActorLocation` _output_get (+ (`self.K2_GetActorLocation` (`self.Spawn`)) (0.0 669.0 100.0)) false true)
  (if (> (`KismetMathLibrary.VSize` (- (`self.K2_GetActorLocation` (`self.Character`)) (`self.K2_GetActorLocation` (`self.Platform`)))) 300.0)
    (`self.K2_SetActorLocation` (`self.Platform`) (`self.K2_GetActorLocation` (`self.Start Position`)) false true)))

(fn `UserConstructionScript`)