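; Blueprint that plays a timed sequence of text reveals when a target actor is overlapped, then destroys two wall actors.
; The overlap sinks this actor, destroys the target and starts a linear chain of Delays.
; Eight referenced text actors are revealed by teleporting them upward rather than toggling visibility.
; The first two drop back down in turn, while the rest stack up in quicker succession, the last also shifting sideways.
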(event `self.Target Actor.OnActorBeginOverlap`
  (params (OverlappedActor :type "Actor Object Reference") (OtherActor :type "Actor Object Reference"))
  (bind _text_4 (`self.Text 4`))
  (bind _text_5 (`self.Text 5`))
  (bind _text_6 (`self.Text 6`))
  (bind _text_7 (`self.Text 7`))
  (bind _text_8 (`self.Text 8`))
  (bind _text_1 (`self.Text 1`))
  (bind _text_2 (`self.Text 2`))
  (bind _text_1_2 (`self.Text 1`))
  (bind _text_2_2 (`self.Text 2`))
  (bind _text_3 (`self.Text 3`))
  (`self.K2_SetActorLocation` (+ (`self.K2_GetActorLocation`) (`KismetMathLibrary.MakeVector` 0.0 0.0 -200.0)) false true)
  (`self.K2_DestroyActor` (`self.Target Actor`))
  (`self.K2_SetActorLocation` _text_1_2 (+ (`self.K2_GetActorLocation` _text_1_2) (`KismetMathLibrary.MakeVector` 0.0 0.0 400.0)) false true)
  (`KismetSystemLibrary.Delay` 7.0)
  (`self.K2_SetActorLocation` _text_1 (+ (`self.K2_GetActorLocation` _text_1) (`KismetMathLibrary.MakeVector` 0.0 0.0 -400.0)) false true)
  (`self.K2_SetActorLocation` _text_2 (+ (`self.K2_GetActorLocation` _text_2) (`KismetMathLibrary.MakeVector` 0.0 0.0 400.0)) false true)
  (`KismetSystemLibrary.Delay` 7.0)
  (`self.K2_SetActorLocation` _text_2_2 (+ (`self.K2_GetActorLocation` _text_2_2) (`KismetMathLibrary.MakeVector` 0.0 0.0 -400.0)) false true)
  (`self.K2_SetActorLocation` _text_3 (+ (`self.K2_GetActorLocation` _text_3) (`KismetMathLibrary.MakeVector` 0.0 0.0 400.0)) false true)
  (`KismetSystemLibrary.Delay` 0.5)
  (`self.K2_SetActorLocation` _text_4 (+ (`self.K2_GetActorLocation` _text_4) (`KismetMathLibrary.MakeVector` 0.0 0.0 400.0)) false true)
  (`KismetSystemLibrary.Delay` 0.5)
  (`self.K2_SetActorLocation` _text_5 (+ (`self.K2_GetActorLocation` _text_5) (`KismetMathLibrary.MakeVector` 0.0 0.0 400.0)) false true)
  (`KismetSystemLibrary.Delay` 0.5)
  (`self.K2_SetActorLocation` _text_6 (+ (`self.K2_GetActorLocation` _text_6) (`KismetMathLibrary.MakeVector` 0.0 0.0 400.0)) false true)
  (`KismetSystemLibrary.Delay` 0.5)
  (`self.K2_SetActorLocation` _text_7 (+ (`self.K2_GetActorLocation` _text_7) (`KismetMathLibrary.MakeVector` 0.0 0.0 400.0)) false true)
  (`KismetSystemLibrary.Delay` 2.0)
  (`self.K2_SetActorLocation` _text_8 (+ (`self.K2_GetActorLocation` _text_8) (`KismetMathLibrary.MakeVector` 0.0 300.0 400.0)) false true)
  (`KismetSystemLibrary.Delay` 2.0)
  (`self.K2_DestroyActor` (`self.Wall1`))
  (`self.K2_DestroyActor` (`self.Wall2`)))

(fn `UserConstructionScript`)