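; BP_Platform is a lift platform that rises while a target actor is near it and can be reset by a button.
; Each tick, if TargetActor is within 200 units, the platform moves up at a constant, frame-rate-independent speed with no upper limit.
; Hitting the referenced Button actor moves the platform straight to the Spawn actor's location without sweeping.
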(event `self.Button.OnActorHit`
  (params (SelfActor :type "Actor Object Reference") (OtherActor :type "Actor Object Reference") (NormalImpulse :type "Vector Structure") (Hit :type "HitResult Structure (by ref)"))
  (`self.K2_SetActorLocation` (`self.K2_GetActorLocation` (`self.Spawn`))))

(event `self.ReceiveTick`
  (params (DeltaSeconds :type "Float (single-precision)"))
  (if (< (`KismetMathLibrary.VSize` (- (`self.K2_GetActorLocation` (`self.Target Actor`)) (`self.K2_GetActorLocation`))) 200.0)
    (`self.K2_SetActorLocation` (+ (`self.K2_GetActorLocation`) (`KismetMathLibrary.MakeVector` 0.0 0.0 (* (`GameplayStatics.GetWorldDeltaSeconds`) 200.0))))))

(fn `UserConstructionScript`)