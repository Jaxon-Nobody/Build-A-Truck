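; BP_LightButton is an interactable actor that lets the player toggle a point light on and off with the Use input.
; On BeginPlay it enables input from the first player controller.
; A box trigger tracks whether something overlaps it and prints an on-screen prompt on entry, without filtering which actor overlaps.
; While overlapped, pressing Use flips a boolean and switches the PointLight intensity between zero and a bright value.
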(event `InputAction|Use`
  (params (Key :type "Key Structure"))
  ;[1 1 1] Turn light on + off
  (:`Pressed`
    (if (`self.Is Overlapped`)
      (if (`self.Is Light On`)
        (`LightComponent.SetIntensity` (`self.PointLight`) 0.0)
        (set `self.Is Light On` false)
        (else
          (`LightComponent.SetIntensity` (`self.PointLight`) 10000.0)
          (set `self.Is Light On` true))))))

(event `self.ReceiveBeginPlay`
  ;[1 1 1] Enable Input
  (`self.EnableInput` (`GameplayStatics.GetPlayerController` 0)))

(event `self.Box.OnComponentBeginOverlap`
  (params (OverlappedComponent :type "PrimitiveComponent Object Reference") (OtherActor :type "Actor Object Reference") (OtherComp :type "PrimitiveComponent Object Reference") (OtherBodyIndex :type Integer) (bFromSweep :type Boolean) (SweepResult :type "HitResult Structure (by ref)"))
  ;[1 1 1] In Range?
  (set `self.Is Overlapped` true)
  (`KismetSystemLibrary.PrintString` "PRESS \"E\"" true true (struct :`R` 1.0 :`B` 1.0 :`A` 1.0)))

(event `self.Box.OnComponentEndOverlap`
  (params (OverlappedComponent :type "PrimitiveComponent Object Reference") (OtherActor :type "Actor Object Reference") (OtherComp :type "PrimitiveComponent Object Reference") (OtherBodyIndex :type Integer))
  ;[1 1 1] In Range?
  (set `self.Is Overlapped` false))

(fn `UserConstructionScript`)